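; Full-sample ACF player character Blueprint that maps input to dodge, attacks, crouch, four quick spells and a companion horse whistle.
; Inputs mostly trigger tagged ACF actions; attacks branch on combat type, with melee trying an execution before a jump or normal attack.
; Component events refresh rotation mode, reset locomotion and aim on riding changes, and toggle the local sprint camera.
; A debug key triggers temporary ragdoll.
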(event OnRidingStateChanged(ACFRider)
  (params (bIsRiding :type Boolean))
  ;[1 1 1] Riding
  (Class|ACFCharacterMovementComponent|ResettoDefaultLocomotionState (Variables|Default|GetLocomotionComp))
  (CallFunction|StopAim))

(event OnCombinedAnimationEnded(ACFExecutor)
  (params (animTag :type Gameplay%20Tag%20Structure%20%28by%20ref%29))
  ;[1 1 1] Reset strafe after exec
  (CallFunction|UpdateRotationMode))

(event ServerCombinedAnimationEnded(ACFExecutor)
  (params (animTag :type Gameplay%20Tag%20Structure%20%28by%20ref%29))
  ;[1 1 1] Reset strafe after exec
  (CallFunction|UpdateRotationMode))

(event OnLocomotionStateChanged(CharacterMovement)
  (params (State :type ELocomotionState%20Enum :default "EIdle"))
  (if (Pawn|IsLocallyControlled)
    (switch Utilities|FlowControl|Switch|SwitchonELocomotionState State
      (:EIdle
        (Class|CCMCameraFunctionLibrary|StopCameraEvent "Sprint" :!label _label))
      (:EWalk
        (goto _label))
      (:EJog
        (goto _label))
      (:ESprint
        (Class|CCMCameraFunctionLibrary|TriggerCameraEvent "Sprint")))))

(event OnMovementModeChangedEvent(CharacterMovement)
  (params (newMovementMode :type EMovementMode%20Enum :default "MOVE_None"))
  (CallFunction|UpdateRotationMode))

(event Input|EnhancedActionEvents|EnhancedInputActionACFQuickSpellInput1
  (params (ActionValue :type Boolean) (ElapsedSeconds :type Float%20%28double-precision%29) (TriggeredSeconds :type Float%20%28double-precision%29) (InputAction :type Input%20Action%20Object%20Reference :default "/AscentCombatFramework/Input/ACFQuickSpellInput1.ACFQuickSpellInput1"))
  ;[1 1 1] Spells
  (Class|ACFActionsManagerComponent|TriggerAction (Variables|Default|GetActionsComp) "(TagName=\"Actions.Fireball\")" "ELow" false))

(event Input|EnhancedActionEvents|EnhancedInputActionACFCrouchInput
  (params (ActionValue :type Boolean) (ElapsedSeconds :type Float%20%28double-precision%29) (TriggeredSeconds :type Float%20%28double-precision%29) (InputAction :type Input%20Action%20Object%20Reference :default "/AscentCombatFramework/Input/ACFCrouchInput.ACFCrouchInput"))
  (if (Variables|Default|GetbIsCrouched)
    (Character|UnCrouch)
    (else
      (Character|Crouch))))

(event Input|EnhancedActionEvents|EnhancedInputActionACFDodgeInput
  (params (ActionValue :type Boolean) (ElapsedSeconds :type Float%20%28double-precision%29) (TriggeredSeconds :type Float%20%28double-precision%29) (InputAction :type Input%20Action%20Object%20Reference :default "/AscentCombatFramework/Input/ACFDodgeInput.ACFDodgeInput"))
  ;[1 1 1] Dodge
  (if (not (Class|ACFRiderComponent|IsRiding (Variables|Default|GetACFRider)))
    (Class|ACFCharacter|TriggerAction "(TagName=\"Actions.Dodge\")" "EMedium" true (Utilities|String|ToString(Vector) (Class|PawnMovementComponent|GetPendingInputVector (Variables|Default|GetLocomotionComp))))))

(event Input|EnhancedActionEvents|EnhancedInputActionACFQuickSpellInput2
  (params (ActionValue :type Boolean) (ElapsedSeconds :type Float%20%28double-precision%29) (TriggeredSeconds :type Float%20%28double-precision%29) (InputAction :type Input%20Action%20Object%20Reference :default "/AscentCombatFramework/Input/ACFQuickSpellInput2.ACFQuickSpellInput2"))
  ;[1 1 1] Spells
  (Class|ACFActionsManagerComponent|TriggerAction (Variables|Default|GetActionsComp) "(TagName=\"Actions.Bless\")" "ELow" false))

(event Input|EnhancedActionEvents|EnhancedInputActionACFQuickSpellInput3
  (params (ActionValue :type Boolean) (ElapsedSeconds :type Float%20%28double-precision%29) (TriggeredSeconds :type Float%20%28double-precision%29) (InputAction :type Input%20Action%20Object%20Reference :default "/AscentCombatFramework/Input/ACFQuickSpellInput3.ACFQuickSpellInput3"))
  ;[1 1 1] Spells
  (Class|ACFActionsManagerComponent|TriggerAction (Variables|Default|GetActionsComp) "(TagName=\"Actions.Summon\")" "ELow" false))

(event Input|EnhancedActionEvents|EnhancedInputActionACFQuickSpellInput4
  (params (ActionValue :type Boolean) (ElapsedSeconds :type Float%20%28double-precision%29) (TriggeredSeconds :type Float%20%28double-precision%29) (InputAction :type Input%20Action%20Object%20Reference :default "/AscentCombatFramework/Input/ACFQuickSpellInput4.ACFQuickSpellInput4"))
  ;[1 1 1] Spells
  (Class|ACFActionsManagerComponent|TriggerAction (Variables|Default|GetActionsComp) "(TagName=\"Actions.AreaSpell\")" "ELow" false))

(event Input|EnhancedActionEvents|EnhancedInputActionACFWhistleInput
  (params (ActionValue :type Boolean) (ElapsedSeconds :type Float%20%28double-precision%29) (TriggeredSeconds :type Float%20%28double-precision%29) (InputAction :type Input%20Action%20Object%20Reference :default "/AscentCombatFramework/Input/ACFWhistleInput.ACFWhistleInput"))
  ;[1 1 1] Horse Whistle: NOTE WORKS ONLY FOR HORSES IN YOUR COMPANIONS GROUP!!!
  (if (not (Variables|Default|GetIsWhistling))
    (Variables|Default|SetIsWhistling true)
    (Audio|PlaySoundatLocation "/Game/FullSample/Assets/SFX/Whistle/whistle_Cue.whistle_Cue" (Transformation|GetActorLocation) "0, 0, 0" 1.0 1.0 0.0 0 0 0 0)
    (Class|ACFGroupAIComponent|SendCommandtoCompanions (Actor|GetComponentbyClass (Class|ACFFunctionLibrary|GetLocalACFPlayerController) "/Script/AIFramework.ACFCompanionGroupAIComponent") "(TagName=\"AICommand.ComeHere\")")
    (Utilities|FlowControl|Delay 2.0)
    (Variables|Default|SetIsWhistling false)))

(event Input|EnhancedActionEvents|EnhancedInputActionACFAttackInput
  (params (ActionValue :type Boolean) (ElapsedSeconds :type Float%20%28double-precision%29) (TriggeredSeconds :type Float%20%28double-precision%29) (InputAction :type Input%20Action%20Object%20Reference :default "/AscentCombatFramework/Input/ACFAttackInput.ACFAttackInput"))
  ;[1 1 1] Attack Action
  (CallFunction|HandleAttackInput))

(event EventBeginPlay
  (|CallParentFunction))

(event Collision|EventActorBeginOverlap
  (params (OtherActor :type Actor%20Object%20Reference))
  (|CallParentFunction OtherActor) ; This node is disabled and will not be called.\nDrag off pins to build functionality.
)

(event Input|KeyboardEvents|DebugKeyB
  (params (Key :type Key%20Structure :default "None") (ActionValue :type Input%20Action%20Value%20Structure))
  (:Pressed
    (Class|ACFRagdollComponent|GoRagdollforDuration (Variables|Default|GetRagdollComp) (Variables|Default|GetImpulse) 2.0)))

(fn ConstructionScript
  (|CallParentFunction))

(fn HandleAttackInput
  (switch Utilities|FlowControl|Switch|SwitchonECombatType (Class|ACFCharacter|GetCombatType)
    (:EUnarmed
      (Class|ACFCharacter|TriggerAction "(TagName=\"Actions.Attack\")" "ELow" true))
    (:EMelee
      (bind _returnvalue (Class|ACFExecutorComponent|TryExecuteCurrentTarget (Variables|Default|GetACFExecutor)))
      (if (not _returnvalue)
        (if (Variables|Default|GetSprintPressed)
          (Class|ACFCharacter|TriggerAction "(TagName=\"Actions.JumpAttack\")" "EMedium" false :!label _label)
          (elif (AI|Components|NavMovement|IsFalling (Variables|Character|GetCharacterMovement))
            (goto _label)
            (else
              (Class|ACFCharacter|TriggerAction "(TagName=\"Actions.Attack\")" "ELow" true))))))))