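; Couch co-op player character that swaps the CCLMT input mapping for the ACF default and tints its mesh through a dynamic material instance.
; Tick reapplies the color, creating a new material instance, and lerps Y toward a locked or limited side-scroller plane.
; Leave input quits the game for player 0; others repossess their input detector, clear their HUD entry and are destroyed.
; Other destructions trigger a GM_CouchCoop respawn when Respawn is set.
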(event Input|EnhancedActionEvents|EnhancedInputActionIA_LeaveGame
  (params (ActionValue :type Boolean) (ElapsedSeconds :type Float%20%28double-precision%29) (TriggeredSeconds :type Float%20%28double-precision%29) (InputAction :type Input%20Action%20Object%20Reference :default "/Game/CouchCoop/Input/Actions/IA_LeaveGame.IA_LeaveGame"))
  (bind _gamemode (Variables|Default|GetGameMode))
  (bind _index (Variables|Default|GetIndex))
  (bind _inputdetectors (Variables|/Game/CouchCoop/Blueprints/GM_CouchCoop.GM_CouchCoop_C|GetInputDetectors _gamemode))
  (bind _output (Utilities|Array|Get(acopy) _inputdetectors _index))
  ;[1 1 1] If player 1 quits quit
  (:Started
    (if (== (Variables|Default|GetIndex) 0)
      (Game|QuitGame 0 "Quit" false)
      (else
        ;[1 1 1] Reposess Input Detector, Remove self from active players and clear Color Selection.
        (Pawn|Possess (Pawn|GetController) _output)
        (Utilities|Array|RemoveItem (Variables|/Game/CouchCoop/Blueprints/GM_CouchCoop.GM_CouchCoop_C|GetActivePlayers _gamemode) self)
        (Variables|/Game/CouchCoop/Blueprints/BP_Input_Detector.BP_Input_Detector_C|SetPlayerChildRef _output 0)
        (Variables|Default|SetRespawn? false)
        (Default|RemovePlayerInfo (Variables|/Game/CouchCoop/Blueprints/GM_CouchCoop.GM_CouchCoop_C|GetInfoHud _gamemode) (Variables|Default|GetIndex) "Visible")
        (Actor|DestroyActor)))))

(event EventBeginPlay
  (bind _index (Variables|Default|GetIndex))
  (bind _returnvalue (Game|GetPlayerController _index))
  (bind _returnvalue_2 (PlayerController|LocalPlayerSubsystems|GetEnhancedInputLocalPlayerSubsystem _returnvalue))
  (|CallParentFunction)
  (Input|RemoveMappingContext _returnvalue_2 "/Game/CouchCoop/Input/CCLMT_MappingContext.CCLMT_MappingContext" "(bIgnoreAllPressedKeysUntilRelease=True,bForceImmediately=False,bNotifyUserSettings=False)")
  (Input|AddMappingContext _returnvalue_2 "/AscentCombatFramework/Input/ACF_DefaultMapping.ACF_DefaultMapping" 0 "(bIgnoreAllPressedKeysUntilRelease=True,bForceImmediately=False,bNotifyUserSettings=False)")
  (bind _asgm_couch_coop (Utilities|Casting|CastToGM_CouchCoop (Game|GetGameMode)))
  (Variables|Default|SetGameMode _asgm_couch_coop)
  (CallFunction|SetupPlayerParameters (Variables|Default|GetColor)))

(event EventTick
  (params (DeltaSeconds :type Float%20%28single-precision%29))
  ;[1 0.5789 0.05237] Event Tick
  (|CallParentFunction DeltaSeconds)
  (CallFunction|SetupPlayerParameters (Variables|Default|GetColor))
  ;;[1 1 1] Side Scroller Y Plane correction and smoothing
  (switch Utilities|FlowControl|Switch|SwitchonEMovementType (Variables|Default|GetMovementType)
    (:NewEnumerator1
      (CallFunction|UpdateYLocked))
    (:NewEnumerator2
      (CallFunction|UpdateYLimited))))

(event EventDestroyed
  (bind _gamemode (Variables|Default|GetGameMode))
  ;[1 1 1] Respawn called on Destroy
  (if (Variables|Default|GetRespawn?)
    (Default|Respawn _gamemode self)
    (Default|MatchStarted _gamemode)))

(event Collision|EventActorBeginOverlap
  (params (OtherActor :type Actor%20Object%20Reference))
  (|CallParentFunction OtherActor) ; This node is disabled and will not be called.\nDrag off pins to build functionality.
)

(fn ConstructionScript
  (|CallParentFunction))

(fn SetupPlayerParameters
  (params (Color :type Linear%20Color%20Structure))
  (bind _returnvalue (Rendering|Material|CreateDynamicMaterialInstance (Variables|Default|GetSkeletalMesh) 0 0 "None" :!class /Script/Engine.PrimitiveComponent))
  (bind _output_get (Variables|Default|SetMatInstance _returnvalue))
  (Rendering|Material|SetVectorParameterValue _output_get "Color" Color :!class /Script/Engine.MaterialInstanceDynamic))

(fn UpdateYLocked
  (bind _returnvalue (Transformation|GetActorLocation))
  (if (!= (.y _returnvalue) 0.0)
    (Transformation|SetActorLocation (Math|Vector|Lerp(Vector) (Transformation|GetActorLocation) (Math|Vector|MakeVector (.x _returnvalue) 0.0 (.z _returnvalue)) (Variables|Default|GetYPlaneSmoothing)) false false)))

(fn UpdateYLimited
  (bind _returnvalue (Transformation|GetActorLocation))
  (bind _returnvalue_2 (Transformation|GetActorLocation))
  ;[1 1 1] Is player in Y limits set?
  (if (not (Math|Float|InRange(Float) (.y _returnvalue) (Variables|Default|GetYPlaneMin) (Variables|Default|GetYPlaneMax)))
    ;[1 1 1] Should we smooth for Upper or Lower Limit
    (if (> (.y _returnvalue) 0.0)
      (Transformation|SetActorLocation (Math|Vector|Lerp(Vector) (Transformation|GetActorLocation) (Math|Vector|MakeVector (.x _returnvalue_2) (Variables|Default|GetYPlaneMax) (.z _returnvalue_2)) (Variables|Default|GetYPlaneSmoothing)) false false)
      (else
        (Transformation|SetActorLocation (Math|Vector|Lerp(Vector) (Transformation|GetActorLocation) (Math|Vector|MakeVector (.x _returnvalue_2) (Variables|Default|GetYPlaneMin) (.z _returnvalue_2)) (Variables|Default|GetYPlaneSmoothing)) false false)))))