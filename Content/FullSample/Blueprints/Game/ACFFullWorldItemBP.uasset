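; World item pickup for the Ascent Combat Framework sample that equips on interaction and drops whatever is left unequipped.
; After the parent interaction and a short delay, it equips the matching inventory item on the ACF character, once only.
; Each unequipped inventory entry loses one count and respawns as a new pickup via chained Server/Client-named events, then this actor destroys itself.
; Its storage component is exposed for saving.
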(event Custom|SpawnNewWorldItemEventClient
  (params (Item%20Class :type ACF%20Item%20Class%20Reference))
  (CallFunction|SpawnNewWorldItem Item%20Class))

(event Custom|SpawnNewWorldItemEventServer
  (params (Item%20Class :type ACF%20Item%20Class%20Reference))
  (CallFunction|SpawnNewWorldItemEventClient Item%20Class))

(event EventBeginPlay
  (|CallParentFunction)
  (Utilities|FlowControl|Delay 0.01)
  (Variables|Default|SetItem (Utilities|Array|Get(acopy) (Class|ACFWorldItem|GetItems))))

(event Collision|EventActorBeginOverlap
  (params (OtherActor :type Actor%20Object%20Reference))
  (|CallParentFunction OtherActor) ; This node is disabled and will not be called.\nDrag off pins to build functionality.
)

(event EventTick
  (params (DeltaSeconds :type Float%20%28single-precision%29))
  (|CallParentFunction DeltaSeconds) ; This node is disabled and will not be called.\nDrag off pins to build functionality.
)

(event EventOnInteractedbyPawn
  (params (Pawn :type Pawn%20Object%20Reference) (interactionType :type String))
  (|CallParentFunction Pawn interactionType)
  (Utilities|FlowControl|Delay 0.25)
  (if (not (Variables|Default|GetItem%20Taken))
    (Variables|Default|SetItem%20Taken true)
    (bind _asacfcharacter (Utilities|Casting|CastToACFCharacter Pawn))
    (Class|ACFEquipmentComponent|EquipItemfromInventory (Class|ACFCharacter|GetEquipmentComponent _asacfcharacter) (.outItem (Class|ACFEquipmentComponent|FindFirstItemOfClassinInventory (Class|ACFCharacter|GetEquipmentComponent _asacfcharacter) (.ItemClass (Utilities|Struct|BreakBaseItem (Variables|Default|GetItem))))))
    (for _array_element (Class|ACFEquipmentComponent|GetInventory (Variables|/Script/AscentCombatFramework.ACFCharacter|GetEquipmentComp _asacfcharacter))
      (if (not (.bIsEquipped (Utilities|Struct|BreakInventoryItem _array_element)))
        (CallFunction|SpawnNewWorldItemEventServer (.itemClass (Utilities|Struct|BreakInventoryItem _array_element)))
        (Class|ACFEquipmentComponent|RemoveItem (Class|ACFCharacter|GetEquipmentComponent _asacfcharacter) _array_element 1)))
    (Actor|DestroyActor)))

(fn ConstructionScript
  (|CallParentFunction))

(fn GetComponentstoSave
  (return (Utilities|Array|MakeArray (Variables|Default|GetStorageComponent))))

(fn SpawnNewWorldItem
  (params (Item%20Class :type ACF%20Item%20Class%20Reference))
  (bind _baseitem (Utilities|Struct|MakeBaseItem Item%20Class 1))
  (bind _returnvalue (Game|SpawnActorfromClass "ACFFullWorldItemBP_C" (Math|Conversions|ToTransform(Vector) (+ (Transformation|GetActorLocation) "0.000000,0.000000,20.000000")) "Undefined" "MultiplyWithRoot" 0 0))
  (Class|ACFStorageComponent|RemoveItems (Variables|/Script/InventorySystem.ACFWorldItem|GetStorageComponent _returnvalue) (Class|ACFStorageComponent|GetItems (Variables|/Script/InventorySystem.ACFWorldItem|GetStorageComponent _returnvalue)))
  (Class|ACFWorldItem|AddItem _returnvalue _baseitem)
  (Variables|ACFFullWorldItemBP_C|SetItem _returnvalue _baseitem))