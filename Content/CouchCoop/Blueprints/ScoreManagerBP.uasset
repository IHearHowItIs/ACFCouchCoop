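; Score manager actor for couch co-op that awards points to player indices through GM_CouchCoop's UpdateScore.
; BeginPlay seeds the award amount from the GameType scoring mode.
; AddPointstoTotal either gives every IndexArray entry except the passed-in loser a fixed award, or scores only the passed index.
; In the ranked modes, the award steps down (Top to Bottom) or up (Bottom to Top) after each call, so call order sets placement.
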(event Custom|Add%20Points%20to%20Total
  (params (Index :type Integer))
  (switch Utilities|FlowControl|Switch|SwitchonEPointGainingType (Variables|Default|GetGameType)
    (:NewEnumerator0
      (bind _asgm_couch_coop (Utilities|Casting|CastToGM_CouchCoop (Game|GetGameMode)))
      (for (_array_element _array_index) (Variables|Default|GetIndexArray)
        (if (!= _array_element Index)
          (Default|UpdateScore _asgm_couch_coop _array_index (Variables|Default|GetPointsToAward)))))
    (:NewEnumerator1
      (bind _asgm_couch_coop_2 (Utilities|Casting|CastToGM_CouchCoop (Game|GetGameMode)))
      (Default|UpdateScore _asgm_couch_coop_2 Index (Variables|Default|GetPointsToAward))
      (bind _result (Math|Integer|DecrementInt (Variables|Default|GetPointsToAward))
        (:%20%20
          (Variables|Default|SetPointsToAward _result))))
    (:NewEnumerator2
      (bind _asgm_couch_coop_3 (Utilities|Casting|CastToGM_CouchCoop (Game|GetGameMode)))
      (Default|UpdateScore _asgm_couch_coop_3 Index (Variables|Default|GetPointsToAward))
      (bind _result_2 (Math|Integer|IncrementInt (Variables|Default|GetPointsToAward))
        (:%20%20
          (Variables|Default|SetPointsToAward _result_2))))))

(event EventBeginPlay
  (switch Utilities|FlowControl|Switch|SwitchonEPointGainingType (Variables|Default|GetGameType)
    (:NewEnumerator0
      (Variables|Default|SetPointsToAward 2))
    (:NewEnumerator1
      (Variables|Default|SetPointsToAward 3))
    (:NewEnumerator2
      (Variables|Default|SetPointsToAward 0))))

(event Collision|EventActorBeginOverlap
  (params (OtherActor :type Actor%20Object%20Reference)))

(event EventTick
  (params (DeltaSeconds :type Float%20%28single-precision%29)))

(fn ConstructionScript)