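; Game manager for a couch co-op stage that tracks player deaths, feeds scoring and decides when the stage ends.
; BeginPlay registers player indices, passes the game type to ScoreManager and derives a death countdown from game type and player count.
; Each death scores that player and decrements the countdown; at zero, Bottom to Top also scores the remaining player.
; Stage end nearly freezes time with global dilation and shows the score widget.
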(event Custom|EndOfStage
  (Utilities|Time|SetGlobalTimeDilation 0.01)
  (bind _returnvalue (UserInterface|CreateWidget "/Game/CouchCoop/UI/BPW_Score.BPW_Score_C"))
  (UserInterface|Viewport|AddtoViewport _returnvalue 0)
  (Utilities|FlowControl|Delay 1e+01))

(event Custom|OnPlayerDeath
  (params (Index :type Integer))
  (Utilities|Array|RemoveItem (Variables|Default|GetWhoScored) Index)
  (Default|AddPointstoTotal (Variables|Default|GetScoreManager) Index)
  (Utilities|Casting|CastToGI_CouchCoop (Game|GetGameInstance))
  (bind _result (Math|Integer|DecrementInt (Variables|Default|GetTimesToScore))
    (:%20%20
      (bind _output_get (Variables|Default|SetTimesToScore _result))
      (if (== _output_get 0)
        (if (Utilities|Enum|NotEqual(Enum) (Variables|Default|GetGameType) "NewEnumerator2")
          (Development|PrintString "Done")
          (else
            (Development|PrintString "SHOULD BE HERE 
")
            (Default|AddPointstoTotal (Variables|Default|GetScoreManager) (Utilities|Array|Get(acopy) (Variables|Default|GetWhoScored)))))
        (CallFunction|EndOfStage)
        (else
          (Development|PrintString "Not Done"))))))

(event EventBeginPlay
  (bind _asgi_couch_coop (Utilities|Casting|CastToGI_CouchCoop (Game|GetGameInstance)))
  (for _index (range 0 (Variables|/Game/CouchCoop/Blueprints/GI_CouchCoop.GI_CouchCoop_C|GetPlayerCount _asgi_couch_coop))
    (Utilities|Array|Insert (Variables|Default|GetWhoScored) _index _index))
  (Variables|/Game/CouchCoop/Blueprints/ScoreManagerBP.ScoreManagerBP_C|SetGameType (Variables|Default|GetScoreManager) (Variables|Default|GetGameType))
  (bind _asgi_couch_coop_2 (Utilities|Casting|CastToGI_CouchCoop (Game|GetGameInstance)))
  (switch Utilities|FlowControl|Switch|SwitchonEPointGainingType (Variables|Default|GetGameType)
    (:NewEnumerator0
      (Variables|Default|SetTimesToScore 1))
    (:NewEnumerator1
      (bind _result (Math|Integer|DecrementInt (Variables|/Game/CouchCoop/Blueprints/GI_CouchCoop.GI_CouchCoop_C|GetPlayerCount _asgi_couch_coop_2))
        (:%20%20
          (Variables|Default|SetTimesToScore _result))))
    (:NewEnumerator2
      (bind _result_2 (Math|Integer|DecrementInt (Variables|/Game/CouchCoop/Blueprints/GI_CouchCoop.GI_CouchCoop_C|GetPlayerCount _asgi_couch_coop_2))
        (:%20%20
          (Variables|Default|SetTimesToScore _result_2))))))

(fn ConstructionScript)